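; AdvancedAI is an enemy AI that runs the AdvancedAITree behavior tree and melee-attacks the player's SushiSlasherBP pawn.
; On BeginPlay it attaches a static mesh to the mesh's SwordSocket.
; Any actor overlap starts an attack that directly subtracts a percentage of the player's max health and briefly raises Attack1.
; AttackProgress gates attacks through a cooldown, after which the attack repeats while the player still overlaps.
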(event `self.ReceiveBeginPlay`
  (`AIController.RunBehaviorTree` (`AIBlueprintHelperLibrary.GetAIController` self) "/Game/AI/AINinja/Blueprints/AdvancedAITree.AdvancedAITree")
  (bind _returnvalue (`AddComponent|NODE_AddStaticMeshComponent-0`))
  (`SceneComponent.K2_AttachToComponent` _returnvalue (`self.Mesh`) "SwordSocket" "SnapToTarget" "KeepRelative" "KeepRelative" true))

(event `self.ReceiveActorBeginOverlap`
  (params (OtherActor :type "Actor Object Reference"))
  (bind _assushi_slasher_bp (cast `/Game/SushiSlasher/Blueprints/SushiSlasherBP` (`Controller.K2_GetPawn` (`GameplayStatics.GetPlayerController` 0))))
  (if (not (`self.AttackProgress`)) :!label _label
    (set `self.Attack1` true)
    (set `self.AttackProgress` true)
    (bind _returnvalue (* (/ (`/Game/SushiSlasher/Blueprints/SushiSlasherBP.PlayerHealthMax` _assushi_slasher_bp) 100.0) 5.0))
    (set `/Game/SushiSlasher/Blueprints/SushiSlasherBP.PlayerHealthValue` (- (`/Game/SushiSlasher/Blueprints/SushiSlasherBP.PlayerHealthValue` _assushi_slasher_bp) _returnvalue) _assushi_slasher_bp)
    (`KismetSystemLibrary.PrintString` (`KismetStringLibrary.Conv_DoubleToString` _returnvalue))
    (`KismetSystemLibrary.Delay` 0.32)
    (set `self.Attack1` false)
    (`KismetSystemLibrary.Delay` 1.0)
    (set `self.AttackProgress` false)
    (if (`self.IsOverlappingActor` _assushi_slasher_bp)
      (goto _label))))

(fn `UserConstructionScript`
  (`parent.UserConstructionScript`))