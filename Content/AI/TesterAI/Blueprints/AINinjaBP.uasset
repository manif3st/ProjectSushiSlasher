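; AINinjaBP is a ninja AI Blueprint that moves toward the player's SushiSlasherBP pawn when it sees it.
; BeginPlay caches player pawn 0 as the chase target, provided it casts to SushiSlasherBP.
; Both Tick and PawnSensing's OnSeePawn run the same check: if AIPerception's sight list contains the player, AIMoveTo heads for them, stopping on overlap.
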(event `self.ReceiveBeginPlay`
  (bind _assushi_slasher_bp (cast `/Game/SushiSlasher/Blueprints/SushiSlasherBP` (`GameplayStatics.GetPlayerPawn` 0)))
  (set `self.Player` _assushi_slasher_bp))

(event `self.ReceiveTick`
  (params (DeltaSeconds :type "Float (single-precision)"))
  (bind _player (`self.Player`))
  (if (`KismetArrayLibrary.Array_Contains` (`AIPerceptionComponent.GetPerceivedActors` (`self.AIPerception`) "/Script/AIModule.AISense_Sight") _player) :!label _label
    (`|AIMoveTo` self (0.0 0.0 0.0) _player 5.0 true)))

(event `self.PawnSensing.OnSeePawn`
  (params (Pawn :type "Pawn Object Reference"))
  (goto _label))

(fn `UserConstructionScript`)